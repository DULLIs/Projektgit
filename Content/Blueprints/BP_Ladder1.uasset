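; Ladder actor for a 2D side-scroller that lets the player climb upward while holding E.
; Tick sets OnLadder from the Box overlap event's cached actors, enabling input in both branches.
; E starts a 0.1-second Delay loop that sets Flying and adds upward movement, restoring Walking on release or leaving the ladder.
; DisLadder subtracts the player's X from itself and is otherwise unused.
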(event OnComponentBeginOverlap(Box)
  (params (OverlappedComponent :type Primitive%20Component%20Object%20Reference) (OtherActor :type Actor%20Object%20Reference) (OtherComp :type Primitive%20Component%20Object%20Reference) (OtherBodyIndex :type Integer) (bFromSweep :type Boolean) (SweepResult :type Hit%20Result%20Structure%20%28by%20ref%29)))

(event EventTick
  (params (DeltaSeconds :type Float%20%28single-precision%29))
  (bind _returnvalue (Game|GetPlayerController 0))
  (Utilities|FlowControl|Sequence
    (:then_0
      (Variables|Default|SetDisLadder (- (.x (Transformation|GetActorLocation (Game|GetPlayerCharacter 0))) (.x (Transformation|GetActorLocation (Game|GetPlayerCharacter 0))))))
    (:then_1
      (if (Collision|IsOverlappingActor (stale OnComponentBeginOverlap(Box) OverlappedComponent) (stale OnComponentBeginOverlap(Box) OtherActor) :!class /Script/Engine.PrimitiveComponent)
        (Variables|Default|SetOnLadder true)
        (Input|EnableInput _returnvalue)
        (else
          (Variables|Default|SetOnLadder false)
          (Input|EnableInput _returnvalue))))))

(event Input|KeyboardEvents|E
  (params (Key :type Key%20Structure))
  (bind _returnvalue (Game|Player|GetPlayerPawn 0))
  (:Pressed
    (if (Variables|Default|GetOnLadder) :!label _label
      (if (Game|Player|IsInputKeyDown (Game|GetPlayerController 0) "E")
        (Pawn|Components|CharacterMovement|SetMovementMode (Variables|/Script/Engine.Character|GetCharacterMovement (Game|GetPlayerCharacter 0)) "MOVE_Flying" 0)
        (Pawn|Input|AddMovementInput _returnvalue (Transformation|GetActorUpVector _returnvalue) (Variables|Default|GetMovmentSpeed) false)
        (Utilities|FlowControl|Delay 0.1)
        (goto _label)
        (else
          _)))
    (Pawn|Components|CharacterMovement|SetMovementMode (Variables|/Script/Engine.Character|GetCharacterMovement (Game|GetPlayerCharacter 0)) "MOVE_Walking" 0)
    (Utilities|Casting|CastTo2DSideScrollerCharacter (Game|GetPlayerCharacter 0))))

(fn ConstructionScript)